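; BP_SPAD is a SPAD sensor array actor that spawns a grid of pixel actors and records intensity images.
; On BeginPlay it spawns SPADPixel actors at its location, fanned in world-space angles derived from FoV and range, each with a row/column-prefixed file name.
; Yaw spans the full horizontal angle, while pitch steps from the top edge down to zero.
; Each Tick exports RT_Inten as a frame-numbered PNG.
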(event EventBeginPlay
  (Variables|Default|SetX_Incre (/ (* (Class|KismetMathLibrary|DegAtan (/ (Variables|Default|GetX_Half_FoV) (Variables|Default|GetRange))) 2.0) (Math|Conversions|ToFloat(Integer) (Variables|Default|GetNum_Cols))))
  (Variables|Default|SetY_Incre (/ (* (Class|KismetMathLibrary|DegAtan (/ (Variables|Default|GetY_Half_FoV) (Variables|Default|GetRange))) 1.0) (Math|Conversions|ToFloat(Integer) (Variables|Default|GetNum_Rows))))
  (for _index (range 0 (Variables|Default|GetNum_Rows))
    (for _index_2 (range 0 (Variables|Default|GetNum_Cols))
      (Game|SpawnActorfromClass "/Game/SPAD/SPADPixel.SPADPixel_C" (Math|Transform|MakeTransform (Transformation|GetActorLocation) (Math|Rotator|MakeRotator 0.0 (- (Class|KismetMathLibrary|DegAtan (/ (Variables|Default|GetY_Half_FoV) (Variables|Default|GetRange))) (* (Math|Conversions|ToFloat(Integer) _index) (Variables|Default|GetY_Incre))) (- (* (Math|Conversions|ToFloat(Integer) _index_2) (Variables|Default|GetX_Incre)) (Class|KismetMathLibrary|DegAtan (/ (Variables|Default|GetX_Half_FoV) (Variables|Default|GetRange)))))) "Undefined" 0 (Utilities|String|Append (Utilities|String|Append (Utilities|String|Append (Utilities|String|ToString(Integer) _index) "_") (Utilities|String|Append (Utilities|String|ToString(Integer) _index_2) "_")) (Variables|Default|GetFile_Name)) 0))))

(event EventTick
  (params (DeltaSeconds :type Float%20%28single-precision%29))
  (bind _output_get (Variables|Default|SetFrame_Count (+ 1 (Variables|Default|GetFrame_Count))))
  (Rendering|ExportRenderTarget "/Game/SPAD/RT_Inten.RT_Inten" (Variables|Default|GetIntensity_Image_File_Path) (Utilities|String|Append (Utilities|String|ToString(Integer) _output_get) ".png")))

(fn ConstructionScript)